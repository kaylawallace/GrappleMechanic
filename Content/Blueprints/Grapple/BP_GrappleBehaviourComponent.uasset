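; BP_GrappleBehaviourComponent is a grapple component for an owning character that, so far, only detects visible grapple targets.
; While the grapple is retracted, each tick runs a sphere overlap within maximum range for GrappleTarget actors on WorldStatic objects.
; A Visibility line trace from the character to each candidate confirms line of sight.
; Visible targets only have their names printed for debugging; no target selection or grapple movement happens here.
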(event `self.ReceiveTick`
  (params (DeltaSeconds :type "Float (single-precision)"))
  (bind _array (`|MakeArray` (`self.OwningCharacter`) :!type "Actor Object Reference"))
  (if (`|EnumEquality` (`self.GrappleState`) "Retracted")
    (bind (_outactors _returnvalue) (`KismetSystemLibrary.SphereOverlapActors` (`Actor.K2_GetActorLocation` (`self.OwningCharacter`)) (`self.MaxGrappleRange`) (`|MakeArray` "ObjectTypeQuery1" :!type "EObjectTypeQuery Enum") "/Script/GrappleHook.GrappleTarget" _array))
    (if _returnvalue
      (for _array_element _outactors
        (bind (_outhit _returnvalue_2) (`KismetSystemLibrary.LineTraceSingle` (`Actor.K2_GetActorLocation` (`self.OwningCharacter`)) (`Actor.K2_GetActorLocation` _array_element) "TraceTypeQuery1" false _array "ForOneFrame"))
        (if _returnvalue_2
          (if (== (`.HitActor` (`GameplayStatics.BreakHitResult` _outhit)) _array_element)
            (`KismetSystemLibrary.PrintString` (`KismetSystemLibrary.GetDisplayName` _array_element) true true (struct :`G` 0.66 :`B` 1.0 :`A` 1.0) 0.0)))))))