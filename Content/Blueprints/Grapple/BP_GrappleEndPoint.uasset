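; BP_GrappleEndPoint is a grapple end point Blueprint that, as written, only visualizes grapple debug data.
; Its construction script draws a green line from start to end location and a red line from the start along the direction vector, both timed.
; It also prints the grapple target's display name.
; BeginPlay is empty, so the graphs contain no grapple movement or attachment logic.
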(event `self.ReceiveBeginPlay`)

(fn `UserConstructionScript`
  (bind _startlocation (`self.StartLocation`))
  (`KismetSystemLibrary.DrawDebugLine` (`self.StartLocation`) (`self.EndLocation`) (struct :`R` 0.015147 :`G` 1.0 :`A` 1.0) 10.0 2.0)
  (`KismetSystemLibrary.DrawDebugLine` _startlocation (+ _startlocation (* (`self.Direction`) 1000.0)) (struct :`R` 1.0 :`G` 0.043376 :`A` 1.0) 10.0 2.0)
  (`KismetSystemLibrary.PrintString` (`KismetSystemLibrary.GetDisplayName` (`self.GrappleTarget`))))